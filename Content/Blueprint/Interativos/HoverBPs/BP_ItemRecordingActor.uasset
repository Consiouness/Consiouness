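; BP_ItemRecordingActor is an item display actor that shows meshes at a standard size and lets the player rotate them by mouse drag.
; SetNewMesh adds a static mesh component under Mesh and resets MeshRoot's rotation.
; UpdatePivotandScale uniformly scales Mesh to fit DesiredExtend, then offsets it toward its bounds center.
; Click start, move and end events turn mouse deltas into world-space pitch and yaw on MeshRoot.
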(event `UpdatePivotandScale`
  (bind _mesh (`self.Mesh`))
  (set `self.CurrentMeshExtend` (`.BoxExtent` (`self.GetActorBounds` false)))
  (`SceneComponent.SetWorldScale3D` (`self.Mesh`) (* (`SceneComponent.K2_GetComponentScale` (`self.Mesh`)) (`KismetMathLibrary.FMin` (/ (.x (`self.DesiredExtend`)) (.x (`self.CurrentMeshExtend`))) (/ (.y (`self.DesiredExtend`)) (.y (`self.CurrentMeshExtend`))) (/ (.z (`self.DesiredExtend`)) (.z (`self.CurrentMeshExtend`))))))
  (`SceneComponent.K2_AddLocalOffset` (`self.Mesh`) (- (`SceneComponent.K2_GetComponentLocation` _mesh) (`KismetSystemLibrary.GetComponentBounds` _mesh)) false false))

(event `OnClickedStart`
  (params (`Mouse Location` :type "Vector2D Structure"))
  (set `self.OnStartRotateLocation` `Mouse Location`)
  (set `self.RotateEnabled?` true))

(event `OnCLickedEnd`
  (params (`Mouse Location` :type "Vector2D Structure"))
  (set `self.RotateEnabled?` false))

(event `ONMouseMove`
  (params (`Mouse Location` :type "Vector2D Structure"))
  (bind (_x _y) (`KismetMathLibrary.BreakVector2D` (- `Mouse Location` (`self.OnStartRotateLocation`))))
  (if (`self.RotateEnabled?`)
    (`SceneComponent.K2_AddWorldRotation` (`self.MeshRoot`) (`KismetMathLibrary.MakeRotator` 0.0 _y (* _x -1.0)) false false)
    (set `self.OnStartRotateLocation` `Mouse Location`)))

(fn `Set New Mesh`
  (params (`Mesh para ver` :type "StaticMesh Object Reference") (`Relative Transform` :type "Transform Structure"))
  (bind _returnvalue (`AddComponent|NODE_AddStaticMeshComponent-0` :`RelativeTransform` `Relative Transform`))
  (`StaticMeshComponent.SetStaticMesh` _returnvalue `Mesh para ver`)
  (`SceneComponent.K2_AttachToComponent` _returnvalue (`self.Mesh`) "None" "KeepRelative" "KeepRelative" "KeepRelative" true)
  (`SceneComponent.K2_SetRelativeRotation` :`self` (`self.MeshRoot`)))

(fn `UserConstructionScript`)