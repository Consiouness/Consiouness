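; Base actor for interactables, with an empty Interact function and construction-time setup of mesh, trigger sphere and UI.
; Trigger overlaps add or remove it from the FirstPersonCharacter's interaction list, skipping additions once a one-time interaction is done.
; ToggleHighlight shows the prompt and inspect hint according to visibility flags.
; CheckSee copies its static meshes into the player's recreated recording actor and opens mouse-driven item preview widgets in UI-only input.
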(event `self.ReceiveBeginPlay`
  (`self.Setup UI Text`))

(event `self.Interaction Trigger.OnComponentBeginOverlap`
  (params (OverlappedComponent :type "PrimitiveComponent Object Reference") (OtherActor :type "Actor Object Reference") (OtherComp :type "PrimitiveComponent Object Reference") (OtherBodyIndex :type Integer) (bFromSweep :type Boolean) (SweepResult :type "HitResult Structure (by ref)"))
  ;[1 1 1] Adiciona ou remove para a lista de atores de interação
  (if (not (`self.InteraçãoUnicaRealizada?`))
    (bind _asfirst_person_character (cast `/Game/FirstPerson/FirstPersonBP/Blueprints/FirstPersonCharacter` OtherActor)
      (:`then`
        (bind _output_get (set `self.Player` _asfirst_person_character))
        (`/Game/FirstPerson/FirstPersonBP/Blueprints/FirstPersonCharacter.Add Interaction` _output_get self)
        (`KismetSystemLibrary.PrintString` "Adicionando  interação"))
      (:`CastFailed`
        (`KismetSystemLibrary.PrintString` "Casting para o personagem falhou")))))

(event `self.Interaction Trigger.OnComponentEndOverlap`
  (params (OverlappedComponent :type "PrimitiveComponent Object Reference") (OtherActor :type "Actor Object Reference") (OtherComp :type "PrimitiveComponent Object Reference") (OtherBodyIndex :type Integer))
  ;[1 1 1] Adiciona ou remove para a lista de atores de interação
  (bind _asfirst_person_character (cast `/Game/FirstPerson/FirstPersonBP/Blueprints/FirstPersonCharacter` OtherActor))
  (bind _output_get (set `self.Player` _asfirst_person_character))
  (`/Game/FirstPerson/FirstPersonBP/Blueprints/FirstPersonCharacter.Remove Interaction` _output_get self))

(fn `Check/See`
  (if (`self.Item é visível?`)
    (if (not (`self.ItemSendoVisto?`))
      (set `self.ItemSendoVisto?` false)
      (`self.CriaAtorHover_ChamaHUD`))))

(fn `CriaAtorHover_ChamaHUD`
  (bind _returnvalue (`GameplayStatics.GetPlayerController` 0))
  (bind _asfirst_person_character (cast `/Game/FirstPerson/FirstPersonBP/Blueprints/FirstPersonCharacter` (`GameplayStatics.GetPlayerPawn` 0)))
  (`self.K2_DestroyActor` (`/Game/FirstPerson/FirstPersonBP/Blueprints/FirstPersonCharacter.RecordingActorRef` _asfirst_person_character))
  (`/Game/FirstPerson/FirstPersonBP/Blueprints/FirstPersonCharacter.Create Recording Actor` _asfirst_person_character)
  (for _array_element (`self.K2_GetComponentsByClass` "/Script/Engine.StaticMeshComponent")
    (bind _asfirst_person_character_2 (cast `/Game/FirstPerson/FirstPersonBP/Blueprints/FirstPersonCharacter` (`GameplayStatics.GetPlayerPawn` 0)))
    (bind _recordingactorref (`/Game/FirstPerson/FirstPersonBP/Blueprints/FirstPersonCharacter.RecordingActorRef` _asfirst_person_character_2))
    (bind _staticmesh (`StaticMeshComponent.StaticMesh` _array_element))
    (`/Game/Blueprint/Interativos/HoverBPs/BP_ItemRecordingActor.Set New Mesh` _recordingactorref _staticmesh (`SceneComponent.GetRelativeTransform` _array_element))
    (`KismetSystemLibrary.PrintString` (`KismetSystemLibrary.GetDisplayName` _staticmesh))
    (`KismetSystemLibrary.PrintString` "Hello"))
  (`/Game/Blueprint/Interativos/HoverBPs/BP_ItemRecordingActor.UpdatePivotandScale` _recordingactorref) ; Corrige o tamanho do objeto
  ;[1 1 1] Cria a UI p/ ver o objeto
  (bind _returnvalue_2 (`|CreateWidget` "/Game/Blueprint/Interativos/HoverBPs/Widget_ItemPreview.Widget_ItemPreview_C" (`GameplayStatics.GetPlayerController` 0)))
  (`UserWidget.AddToViewport` _returnvalue_2 0)
  (`WidgetBlueprintLibrary.SetInputMode_UIOnlyEx` (`GameplayStatics.GetPlayerController` 0) _returnvalue_2)
  ;[1 1 1] Mostra o mouse e ativa os eventos de click
  (bind _asfirst_person_character_3 (cast `/Game/FirstPerson/FirstPersonBP/Blueprints/FirstPersonCharacter` (`GameplayStatics.GetPlayerPawn` 0)))
  (set `PlayerController.bShowMouseCursor` true _returnvalue)
  (set `PlayerController.bEnableMouseOverEvents` true _returnvalue)
  (set `PlayerController.bEnableClickEvents` true _returnvalue)
  (set `/Game/Blueprint/Interativos/HoverBPs/Widget_ItemPreview.ItemPreviewActorRef` (`/Game/FirstPerson/FirstPersonBP/Blueprints/FirstPersonCharacter.RecordingActorRef` _asfirst_person_character_3) _returnvalue_2) ; Seta o objeto sendo gravado
  (bind _returnvalue_3 (`|CreateWidget` "/Game/Blueprint/Interativos/HoverBPs/Widget_CheckSeeVoltar.Widget_CheckSeeVoltar_C" (`GameplayStatics.GetPlayerController` 0)))
  (`UserWidget.AddToViewport` _returnvalue_3 0))

(fn `Interact`)

(fn `Setup Interaction Trigger`
  (`SphereComponent.SetSphereRadius` (`self.Interaction Trigger`) (`self.TriggerRadius`) true)
  (`SceneComponent.K2_SetRelativeLocation` (`self.Interaction Trigger`) (`self.TriggerOffset`) false false))

(fn `Setup Mesh`
  (`StaticMeshComponent.SetStaticMesh` (`self.Interaction Mesh`) (`self.Actor Mesh`))
  (`SceneComponent.K2_SetRelativeLocation` (`self.Interaction Mesh`) (`self.Mesh Offset`) false false)
  (`SceneComponent.SetWorldScale3D` (`self.Interaction Mesh`) (`self.Mesh Scale`)))

(fn `Setup UI Text`
  (bind _aswidget_interactive_actors (cast `/Game/Blueprint/Interativos/Widget_Interactive_Actors` (`WidgetComponent.GetUserWidgetObject` (`self.Interaction UI`))))
  (`/Game/Blueprint/Interativos/Widget_Interactive_Actors.Set Interaction Text` _aswidget_interactive_actors (`self.UI Description`)))

(fn `SetupInteractionUI`
  (bind _uioffset (`self.UIOffset`))
  (`SceneComponent.K2_SetRelativeLocation` (`self.Interaction UI`) _uioffset false false)
  (`SceneComponent.K2_SetRelativeLocation` (`self.Check/See UI`) (+ _uioffset (60.0 60.0 0.0)) false false))

(fn `Toggle Highlight`
  (params (Highlight :type Boolean))
  (if (`self.Sumir UI da Interação?`)
    (if (`self.Item é visível?`)
      (`SceneComponent.SetVisibility` (`self.Check/See UI`) Highlight false))
    (else
      (`SceneComponent.SetVisibility` (`self.Interaction UI`) Highlight false)
      (if (`self.Item é visível?`)
        (`SceneComponent.SetVisibility` (`self.Check/See UI`) Highlight false)))))

(fn `UserConstructionScript`
  (`self.SetupInteractionUI`)
  (`self.Setup Interaction Trigger`)
  (`self.Setup Mesh`))