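; Interactable alphabet puzzle in which the player drags static mesh pieces into place with the mouse.
; Interact toggles between first person and the puzzle's view, switching cinematic mode, cursor and AlfabetoAuxiliar widget.
; Tick moves the held piece via cursor traces at raised height; release snaps it to relative origin within tolerance.
; Each snap checks all pieces; once solved, it restores player control and replaces itself with Puzzle_Afabeto_Completo.
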(event `self.Interact`
  (bind _returnvalue (`GameplayStatics.GetPlayerController` 0))
  (bind _returnvalue_2 (`GameplayStatics.GetPlayerController` 0))
  (bind _returnvalue_3 (`GameplayStatics.GetPlayerController` 0))
  (`parent.Interact`)
  (if (not (`self.InteraçãoAcontecendo?`))
    (set `self.InteraçãoAcontecendo?` true)
    (`self.Toggle Highlight` false)
    ;[1 1 1] Define se é para entrar ou sair
    (if (`self.QuerSairDoALfabeto?`)
      (bind _asfirst_person_character (cast `/Game/FirstPerson/FirstPersonBP/Blueprints/FirstPersonCharacter` (`GameplayStatics.GetPlayerPawn` 0)))
      (`PlayerController.SetViewTargetWithBlend` (`GameplayStatics.GetPlayerController` 0) _asfirst_person_character 0.0 "VTBlend_Linear" 0.0 false)
      (set `self.QuerSairDoALfabeto?` false)
      (`PlayerController.SetCinematicMode` (`GameplayStatics.GetPlayerController` 0) false false true true true)
      (set `PlayerController.bShowMouseCursor` false _returnvalue_2)
      (`WidgetBlueprintLibrary.SetInputMode_GameOnly` _returnvalue_2)
      (set `PlayerController.bEnableMouseOverEvents` false _returnvalue_2)
      (set `self.InteraçãoAcontecendo?` false)
      (set `self.UI Description` "RESOLVER")
      (set `self.UIOffset` (0.0 0.0 50.0))
      (`self.Setup UI Text`)
      (`self.SetupInteractionUI`)
      (`self.Toggle Highlight` true)
      (bind _foundwidgets (`WidgetBlueprintLibrary.GetAllWidgetsOfClass` "/Game/Assets/Alfabeto/Import/AlfabetoAuxiliar.AlfabetoAuxiliar_C"))
      (`Widget.RemoveFromParent` _foundwidgets)
      (else
        ;[1 1 1] Seta a visão, a variável de controle para saida e arruma a UI do objeto
        (`PlayerController.SetCinematicMode` _returnvalue true true true true true)
        (`PlayerController.SetViewTargetWithBlend` _returnvalue self 0.0 "VTBlend_Linear" 0.0 false)
        (set `self.QuerSairDoALfabeto?` true)
        (set `self.UI Description` "SAIR")
        (set `self.UIOffset` (200.0 125.0 0.0))
        (`self.Setup UI Text`)
        (`self.SetupInteractionUI`)
        (`self.Toggle Highlight` true)
        (set `self.InteraçãoAcontecendo?` false)
        ;[1 1 1] Mostra o mouse e ativa os eventos de click
        (cast `/Game/FirstPerson/FirstPersonBP/Blueprints/FirstPersonCharacter` (`GameplayStatics.GetPlayerPawn` 0))
        (set `PlayerController.bShowMouseCursor` true _returnvalue_3)
        (set `PlayerController.bEnableMouseOverEvents` true _returnvalue_3)
        (set `PlayerController.bEnableClickEvents` true _returnvalue_3)
        (bind _returnvalue_4 (`|CreateWidget` "/Game/Assets/Alfabeto/Import/AlfabetoAuxiliar.AlfabetoAuxiliar_C" (`GameplayStatics.GetPlayerController` 0)))
        (`UserWidget.AddToViewport` _returnvalue_4 0)))))

(event `self.ReceiveTick`
  (params (DeltaSeconds :type "Float (single-precision)"))
  (bind _hitresult (`PlayerController.GetHitResultUnderCursorByChannel` (`GameplayStatics.GetPlayerController` 0) "TraceTypeQuery1" true))
  (if (`self.QuerSairDoALfabeto?`)
    (if (`self.Está Cliclado?`)
      (set `PlayerController.CurrentMouseCursor` "GrabHandClosed" (`GameplayStatics.GetPlayerController` 0))
      (bind _returnvalue (+ (`KismetMathLibrary.MakeVector` (.x (`.Location` (`GameplayStatics.BreakHitResult` _hitresult))) (.y (`.Location` (`GameplayStatics.BreakHitResult` _hitresult))) (+ (`self.Posição_Z_Inicial`) (`self.Altura_Z_Grabado`))) (stale `self.ReceiveActorOnClicked` _output_get_2)))
      (`SceneComponent.K2_SetWorldLocation` (`self.ComponenteInicial`) _returnvalue false false)
      (set `self.Posição_Final` _returnvalue)
      (set `self.UltimoComponenteMovido` (`.HitComponent` (`GameplayStatics.BreakHitResult` _hitresult)))
      (elif (>= (`KismetArrayLibrary.Array_Find` (`self.TodosComponentes`) (`.HitComponent` (`GameplayStatics.BreakHitResult` (`PlayerController.GetHitResultUnderCursorByChannel` (`GameplayStatics.GetPlayerController` 0) "TraceTypeQuery2" true)))) 0)
        (set `PlayerController.CurrentMouseCursor` "Hand" (`GameplayStatics.GetPlayerController` 0))
        (else
          (set `PlayerController.CurrentMouseCursor` "Default" (`GameplayStatics.GetPlayerController` 0)))))))

(event `self.ReceiveActorOnClicked`
  (params (ButtonPressed :type "Key Structure"))
  (bind _hitresult (`PlayerController.GetHitResultUnderCursorByChannel` (`GameplayStatics.GetPlayerController` 0) "TraceTypeQuery1" true))
  (set `self.Está Cliclado?` true :!label _label)
  (if (>= (`KismetArrayLibrary.Array_Find` (`self.TodosComponentes`) (`.HitComponent` (`GameplayStatics.BreakHitResult` _hitresult))) 0)
    (bind _output_get (set `self.ComponenteInicial` (`.HitComponent` (`GameplayStatics.BreakHitResult` _hitresult))))
    (bind _output_get_2 (set `self.Offset` (- (`SceneComponent.K2_GetComponentLocation` (`.HitComponent` (`GameplayStatics.BreakHitResult` _hitresult))) (`.Location` (`GameplayStatics.BreakHitResult` _hitresult)))))))

(event `self.ReceiveActorOnInputTouchBegin`
  (params (FingerIndex :type "ETouchIndex Enum" :default "Touch1"))
  (goto _label))

(event `self.ReceiveActorOnReleased`
  (params (ButtonReleased :type "Key Structure"))
  (set `self.Está Cliclado?` false :!label _label_2)
  (`self.SnapPraPosição` (stale `self.ReceiveActorOnClicked` _output_get))
  (set `self.ComponenteInicial` null))

(event `self.ReceiveActorOnInputTouchEnd`
  (params (FingerIndex :type "ETouchIndex Enum" :default "Touch1"))
  (goto _label_2))

(fn `SnapPraPosição`
  (params (ComponenteALevarOSnap :type "PrimitiveComponent Object Reference"))
  (if (== (`SceneComponent.RelativeLocation` ComponenteALevarOSnap) (0.0 0.0 0.0) :`ErrorTolerance` (`self.Tolerância_Snap`))
    (`SceneComponent.K2_SetRelativeLocation` ComponenteALevarOSnap (0.0 0.0 0.0) false false)
    (`self.VerificaTodosPosição`)))

(fn `UserConstructionScript`
  (`parent.UserConstructionScript`)
  (set `self.Posição_Z_Inicial` (.z (`self.K2_GetActorLocation`)))
  (bind _output_get (set `self.TodosComponentes` (`self.K2_GetComponentsByClass` "/Script/Engine.StaticMeshComponent")))
  (`KismetArrayLibrary.Array_RemoveItem` _output_get (`self.Alfabeto_completo`)))

(fn `VerificaTodosPosição`
  (bind _returnvalue (`GameplayStatics.GetPlayerController` 0))
  (`KismetArrayLibrary.Array_Clear` (`self.TudoNaPosiçãoArray`))
  (for _array_element (`self.TodosComponentes`)
    (bind _returnvalue_2 (== (`SceneComponent.RelativeLocation` _array_element) (0.0 0.0 0.0)))
    (if (not _returnvalue_2)
      (`KismetArrayLibrary.Array_AddUnique` (`self.TudoNaPosiçãoArray`) _returnvalue_2)))
  (if (not (`KismetArrayLibrary.Array_Contains` (`self.TudoNaPosiçãoArray`)))
    (`KismetSystemLibrary.PrintString` "Parabéns Caralho!!!")
    (bind _asfirst_person_character (cast `/Game/FirstPerson/FirstPersonBP/Blueprints/FirstPersonCharacter` (`GameplayStatics.GetPlayerPawn` 0)))
    (`PlayerController.SetViewTargetWithBlend` (`GameplayStatics.GetPlayerController` 0) _asfirst_person_character 0.0 "VTBlend_Linear" 0.0 false)
    (set `self.QuerSairDoALfabeto?` false)
    (`PlayerController.SetCinematicMode` (`GameplayStatics.GetPlayerController` 0) false false true true true)
    (set `PlayerController.bShowMouseCursor` false _returnvalue)
    (`WidgetBlueprintLibrary.SetInputMode_GameOnly` _returnvalue)
    (set `PlayerController.bEnableMouseOverEvents` false _returnvalue)
    (set `self.InteraçãoAcontecendo?` false)
    (set `self.UI Description` "RESOLVER")
    (set `self.UIOffset` (0.0 0.0 50.0))
    (`self.Setup UI Text`)
    (`self.SetupInteractionUI`)
    (`self.Toggle Highlight` true)
    (bind _foundwidgets (`WidgetBlueprintLibrary.GetAllWidgetsOfClass` null))
    (`Widget.RemoveFromParent` _foundwidgets)
    (bind _output_get (set `self.Transform_Destruição` (`self.GetTransform`)))
    (`self.K2_DestroyActor`)
    (`|SpawnActorFromClass` "/Game/Blueprint/Interativos/Puzzle_Afabeto_Completo.Puzzle_Afabeto_Completo_C" _output_get "Undefined" "OverrideRootScale" null null)))